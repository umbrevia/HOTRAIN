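; BP_GameState_Hotrain is the game state that handles the switch from game open to active play.
; On BeginPlay it applies a muted environment sound mix through OnGameOpen.
; OnGameStart restores environment audio, spawns BP_PlayerCharacter at a PlayerStart, then possesses it, hides the cursor and sets game-only input.
; Nothing in this Blueprint calls OnGameStart, and its percent math expression is unused.
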(event EventOnGameStart
  (bind _returnvalue (Game|GetPlayerController 0))
  (Class|GameplayStatics|SetBaseSoundMix "/Game/Sounds/Island/SCM_EnvironmentUnmute.SCM_EnvironmentUnmute")
  (bind _returnvalue_2 (Actor|GetActorOfClass "/Script/Engine.PlayerStart"))
  (bind _returnvalue_3 (Game|SpawnActorfromClass "/Game/Blueprints/Characters/Player/BP_PlayerCharacter.BP_PlayerCharacter_C" (Transformation|GetActorTransform _returnvalue_2) "Undefined" "MultiplyWithRoot" 0 0))
  (Utilities|IsValid _returnvalue_3
    (:Is%20Valid
      (Pawn|Possess _returnvalue _returnvalue_3)
      (Variables|/Script/Engine.PlayerController|SetbShowMouseCursor _returnvalue false)
      (Input|SetInputModeGameOnly _returnvalue false))))

(event EventOnGameOpen
  (Class|GameplayStatics|SetBaseSoundMix "/Game/Sounds/Island/SCM_EnvironmentMute.SCM_EnvironmentMute"))

(event EventBeginPlay
  (CallFunction|OnGameOpen))

(fn ConstructionScript)