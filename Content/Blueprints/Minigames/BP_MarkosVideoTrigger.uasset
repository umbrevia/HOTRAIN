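; Trigger box minigame that plays the Markos video when the player character overlaps it.
; On overlap it hides the objective FX, swaps ambient audio to the Markos track, blends to a dedicated camera, disables input and plays the media.
; After a fixed five-second delay, not tied to video end, it restores view and input, sets jazz-funk music and flags completion.
; Leaving the box re-shows the FX only while unfinished.
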(event OnComponentBeginOverlap(Box)
  (params (OverlappedComponent :type Primitive%20Component%20Object%20Reference) (OtherActor :type Actor%20Object%20Reference) (OtherComp :type Primitive%20Component%20Object%20Reference) (OtherBodyIndex :type Integer) (bFromSweep :type Boolean) (SweepResult :type Hit%20Result%20Structure%20%28by%20ref%29))
  (bind _returnvalue (Game|GetPlayerController 0))
  (bind _mediaplayer (Variables|Default|GetMediaPlayer))
  (CallFunction|OnMiniGameStarted)
  (bind _asbp_player_character (Utilities|Casting|CastToBP_PlayerCharacter OtherActor))
  (bind _output_get (Variables|Default|SetRef_PlayerCharacter _asbp_player_character))
  (Input|DisableInput _output_get (Game|GetPlayerController 0))
  (Media|MediaPlayer|OpenSourcewithOptions _mediaplayer "/Game/Movies/FMS_Markos.FMS_Markos" (Utilities|Struct|MakeMediaPlayerOptions "(Audio=0,Caption=-1,Metadata=-1,Script=-1,Subtitle=-1,Text=-1,Video=0)" "UseTrackOptionIndices" "+00000000.00:00:00.000000000" "RelativeToStartTime" "UseMediaPlayerSetting" "Enabled") :!class /Script/MediaAssets.MediaPlayer)
  (EventDispatchers|AssignOnMediaOpened _mediaplayer (delegate Custom|OnMediaOpened_Event))
  (Utilities|FlowControl|Delay 5.0)
  (bind _ref_playercharacter (Variables|Default|GetRef_PlayerCharacter)
    (:then
      (Game|Player|SetViewTargetwithBlend _returnvalue _ref_playercharacter 1.0 "VTBlend_Linear" 0.0 false)
      (Input|EnableInput _ref_playercharacter _returnvalue)
      (Audio|Components|Audio|SetSound (Variables|/Script/Engine.AmbientSound|GetAudioComponent (Variables|Default|GetAmbientAudio_Ref)) "/Game/Sounds/Restaurant/jazz_funk_fusion_in_b_minor_by_yohan_kim_edit.jazz_funk_fusion_in_b_minor_by_yohan_kim_edit")
      (Variables|Default|SetbIsGameFinished true))
    (:else)))

(event OnComponentEndOverlap(Box)
  (params (OverlappedComponent :type Primitive%20Component%20Object%20Reference) (OtherActor :type Actor%20Object%20Reference) (OtherComp :type Primitive%20Component%20Object%20Reference) (OtherBodyIndex :type Integer))
  (if (not (Variables|Default|GetbIsGameFinished))
    (Rendering|SetVisibility (Variables|Default|GetObjectiveFX) true false)))

(event Custom|OnMiniGameStarted
  (Rendering|SetVisibility (Variables|Default|GetObjectiveFX) false false)
  (bind _ambientaudio_ref (Variables|Default|GetAmbientAudio_Ref)
    (:then
      (Audio|Components|Audio|SetSound (Variables|/Script/Engine.AmbientSound|GetAudioComponent _ambientaudio_ref) "/Game/Sounds/Restaurant/markos_ai_edit_2_final_audio.markos_ai_edit_2_final_audio")
      (bind _markoscamera_ref (Variables|Default|GetMarkosCamera_Ref)
        (:then
          (Game|Player|SetViewTargetwithBlend (Game|GetPlayerController 0) _markoscamera_ref 1.0 "VTBlend_Linear" 0.0 false))
        (:else)))
    (:else)))

(event Custom|OnMediaOpened_Event
  (params (OpenedUrl :type String))
  (Media|MediaPlayer|Play (Variables|Default|GetMediaPlayer) :!class /Script/MediaAssets.MediaPlayer))

(fn ConstructionScript)