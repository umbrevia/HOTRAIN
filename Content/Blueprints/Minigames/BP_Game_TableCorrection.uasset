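; Table-correction minigame actor where the player straightens a chair and a knife by clicking world widget buttons.
; Overlapping the box blends the camera to this actor, shows both buttons and switches to UI-only input.
; Each click adds a fixed yaw step while below target, playing a sound on an exact match.
; Tick polls both yaws with exact float equality, then completes once, hiding buttons and restoring player view and input.
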(event OnComponentBeginOverlap(Box)
  (params (OverlappedComponent :type Primitive%20Component%20Object%20Reference) (OtherActor :type Actor%20Object%20Reference) (OtherComp :type Primitive%20Component%20Object%20Reference) (OtherBodyIndex :type Integer) (bFromSweep :type Boolean) (SweepResult :type Hit%20Result%20Structure%20%28by%20ref%29))
  (if (not (Variables|Default|GetbIsMinigameCompleted))
    (CallFunction|OnGameStarted OtherActor)))

(event OnComponentEndOverlap(Box)
  (params (OverlappedComponent :type Primitive%20Component%20Object%20Reference) (OtherActor :type Actor%20Object%20Reference) (OtherComp :type Primitive%20Component%20Object%20Reference) (OtherBodyIndex :type Integer))
  (if (not (Variables|Default|GetbIsMinigameCompleted))
    (Rendering|SetVisibility (Variables|Default|GetObjectiveFX) true false)))

(event Custom|Event_OnButtonClickedChair
  (CallFunction|RotateGameObjects (Variables|Default|GetChair) (Variables|Default|GetTargetRotationChair) 2e+01))

(event Custom|Event_OnButtonClickedKnife
  (CallFunction|RotateGameObjects (Variables|Default|GetKnife) (Variables|Default|GetTargetRotationKnife) 3e+01))

(event Custom|OnGameCompleted
  (Rendering|SetVisibility (Variables|Default|GetRotateChair) false false)
  (Variables|Default|SetbIsMinigameCompleted true)
  (bind _ref_playercharacter (Variables|Default|GetRef_PlayerCharacter)
    (:then
      (CallFunction|AdjustView _ref_playercharacter "NewEnumerator1")
      (Variables|Default|SetRef_PlayerCharacter 0))
    (:else)))

(event Custom|OnGameStarted
  (params (OtherActor :type Actor%20Object%20Reference))
  (Rendering|SetVisibility (Variables|Default|GetObjectiveFX) false false)
  (Rendering|SetVisibility (Variables|Default|GetRotateChair) true false)
  (bind _asbp_player_character (Utilities|Casting|CastToBP_PlayerCharacter OtherActor))
  (Variables|Default|SetRef_PlayerCharacter _asbp_player_character)
  (CallFunction|AdjustView self "NewEnumerator0"))

(event EventBeginPlay
  (bind _aswbp_interactable_img_button (Utilities|Casting|CastToWBP_Interactable_Img_Button (UserInterface|GetUserWidgetObject (Variables|Default|GetRotateChair))))
  (EventDispatchers|BindEventtoOnClickButton _aswbp_interactable_img_button (delegate Custom|Event_OnButtonClickedChair))
  (bind _aswbp_interactable_img_button_2 (Utilities|Casting|CastToWBP_Interactable_Img_Button (UserInterface|GetUserWidgetObject (Variables|Default|GetRotateKnife))))
  (EventDispatchers|BindEventtoOnClickButton _aswbp_interactable_img_button_2 (delegate Custom|Event_OnButtonClickedKnife)))

(event EventTick
  (params (DeltaSeconds :type Float%20%28single-precision%29))
  (if (and (CallFunction|CheckifObjectsAlignedCorrectly (Variables|Default|GetKnife) (Variables|Default|GetTargetRotationKnife)) (CallFunction|CheckifObjectsAlignedCorrectly (Variables|Default|GetChair) (Variables|Default|GetTargetRotationChair)))
    (Utilities|FlowControl|DoOnce false
      (:Completed
        (CallFunction|OnGameCompleted)))))

(fn ConstructionScript)

(fn AdjustView
  (params (NewViewTarget :type Actor%20Object%20Reference) (MinigameState :type E_MinigameState%20Enum :default "NewEnumerator0"))
  (bind _returnvalue (Game|GetPlayerController 0))
  (bind _returnvalue_2 (Game|GetPlayerController 0))
  (Game|Player|SetViewTargetwithBlend _returnvalue NewViewTarget 1.0 "VTBlend_Linear" 0.0 false)
  (switch Utilities|FlowControl|Switch|SwitchonE_MinigameState MinigameState
    (:NewEnumerator0
      (Variables|/Script/Engine.PlayerController|SetbShowMouseCursor _returnvalue true)
      (Input|SetInputModeUIOnly _returnvalue (UserInterface|GetWidget (Variables|Default|GetRotateKnife)) "DoNotLock" false))
    (:NewEnumerator1
      (Variables|/Script/Engine.PlayerController|SetbShowMouseCursor _returnvalue_2 false)
      (Input|SetInputModeGameOnly _returnvalue_2 false))))

(fn RotateGameObjects
  (params (GameObject :type Static%20Mesh%20Component%20Object%20Reference) (TargetRotation :type Float%20%28double-precision%29) (RotationAddAmount :type Float%20%28double-precision%29))
  (bind _relativerotation (Variables|/Script/Engine.SceneComponent|GetRelativeRotation GameObject))
  (bind _relativerotation_2 (Variables|/Script/Engine.SceneComponent|GetRelativeRotation GameObject))
  (if (< (.yaw _relativerotation_2) TargetRotation)
    (Transformation|SetRelativeRotation GameObject (Math|Rotator|MakeRotator 0.0 0.0 (+ (.yaw _relativerotation_2) RotationAddAmount)) false false)
    (if (== (.yaw _relativerotation) TargetRotation)
      (Audio|PlaySoundatLocation "/Game/Sounds/Restaurant/diamond_collect.diamond_collect" (Transformation|GetActorLocation) "0, 0, 0" 1.0 1.0 0.0 0 0 0 0)
      (Development|PrintString (Utilities|String|ToString(Float) (.yaw _relativerotation))))))

(fn CheckifObjectsAlignedCorrectly
  (params (MeshComponent :type Static%20Mesh%20Component%20Object%20Reference) (TargetRotationValue :type Float%20%28double-precision%29))
  (return (== (.yaw (Variables|/Script/Engine.SceneComponent|GetRelativeRotation MeshComponent)) TargetRotationValue)))