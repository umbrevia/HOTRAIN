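; BPC_MovementComponent is a character component that switches its owning BP_CharacterBase between walking and running speeds.
; On BeginPlay it casts and caches the owner, then sets the character movement's max walk speed to the walk speed.
; SetMovementState takes a movement state and, if the cached owner is valid, applies either the walk or run speed to the movement component.
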(event EventBeginPlay
  (bind _asbp_character_base (Utilities|Casting|CastToBP_CharacterBase (Components|GetOwner)))
  (bind _output_get (Variables|Default|SetCharacterOwner _asbp_character_base))
  (Variables|/Script/Engine.CharacterMovementComponent|SetMaxWalkSpeed (Variables|/Script/Engine.Character|GetCharacterMovement _output_get) (Variables|Default|GetWalkSpeed)))

(fn SetMovementState
  (params (NewState :type E_MovementState%20Enum :default "NewEnumerator0"))
  (switch Utilities|FlowControl|Switch|SwitchonE_MovementState NewState
    (:NewEnumerator0
      (bind _characterowner (Variables|Default|GetCharacterOwner)
        (:then
          (Variables|/Script/Engine.CharacterMovementComponent|SetMaxWalkSpeed (Variables|/Script/Engine.Character|GetCharacterMovement _characterowner) (Variables|Default|GetWalkSpeed)))
        (:else)))
    (:NewEnumerator1
      (bind _characterowner_2 (Variables|Default|GetCharacterOwner)
        (:then
          (Variables|/Script/Engine.CharacterMovementComponent|SetMaxWalkSpeed (Variables|/Script/Engine.Character|GetCharacterMovement _characterowner_2) (Variables|Default|GetRunSpeed)))
        (:else)))))