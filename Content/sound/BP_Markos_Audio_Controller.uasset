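; Audio controller actor with a resizable trigger box that switches between restaurant ambience plus jazz and a Markos track.
; BeginPlay starts ambience and jazz; entering the box starts Markos and the volume timelines for all three sounds.
; Leaving the box or the continue event reverses those timelines, replays the background and sets MissionFailed.
; Other events stop or resume the background; a delayed sound gated on MissionFailed is unwired.
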(event OnComponentBeginOverlap(Box)
  (params (OverlappedComponent :type Primitive%20Component%20Object%20Reference) (OtherActor :type Actor%20Object%20Reference) (OtherComp :type Primitive%20Component%20Object%20Reference) (OtherBodyIndex :type Integer) (bFromSweep :type Boolean) (SweepResult :type Hit%20Result%20Structure%20%28by%20ref%29))
  (bind _markos (Variables|Default|GetMarkos))
  (Class|AudioComponent|SetPaused _markos false)
  (Audio|Components|Audio|SetVolumeMultiplier _markos 0.5 :!class /Script/Engine.AudioComponent)
  (Audio|Components|Audio|Play _markos 0.0)
  (Audio|Components|Audio|Play (Variables|Default|GetMarkosTimeline))
  (Utilities|FlowControl|Delay 0.2)
  (Components|Timeline|PlayfromStart (Variables|Default|GetAmbienceTimeline_0)))

(event OnComponentEndOverlap(Box)
  (params (OverlappedComponent :type Primitive%20Component%20Object%20Reference) (OtherActor :type Actor%20Object%20Reference) (OtherComp :type Primitive%20Component%20Object%20Reference) (OtherBodyIndex :type Integer))
  (Class|AudioComponent|SetPaused (Variables|Default|GetRestaurantAmbience) false)
  (Utilities|String|Reverse (Variables|Default|GetMarkosTimeline))
  (Audio|Components|Audio|Play (Variables|Default|GetRestaurantAmbience) 0.0)
  (Variables|Default|SetbMissionFailed true))

(event Custom|Event_OnSoundStop
  (Audio|Components|Audio|Play (Variables|Default|GetJazzTimeline_1)))

(event Custom|YeniSound_Stop
  (bind _restaurantambience (Variables|Default|GetRestaurantAmbience))
  (bind _jazzsound (Variables|Default|GetJazzSound))
  (Class|AudioComponent|SetPaused _restaurantambience true)
  (if (and (Audio|Components|Audio|IsPlaying _restaurantambience) (Audio|Components|Audio|IsPlaying _jazzsound))
    (Audio|Components|Audio|Stop _jazzsound)))

(event Custom|Event_OnSoundPlay
  (Class|AudioComponent|SetPaused (Variables|Default|GetRestaurantAmbience) false)
  (Audio|Components|Audio|Play (Variables|Default|GetJazzSound) 0.0))

(event Custom|Event_OnSoundContinue
  (Utilities|String|Reverse (Variables|Default|GetMarkosTimeline))
  (Audio|Components|Audio|Play (Variables|Default|GetRestaurantAmbience) 0.0)
  (Variables|Default|SetbMissionFailed true))

(event Custom|YeniSound_JazzOn
  (bind _jazzsound (Variables|Default|GetJazzSound))
  (Class|AudioComponent|SetPaused _jazzsound false)
  (Audio|Components|Audio|Play _jazzsound 0.0))

(event EventBeginPlay
  (Class|AudioComponent|SetPaused (Variables|Default|GetRestaurantAmbience) false)
  (Audio|Components|Audio|Play (Variables|Default|GetJazzSound) 0.0))

(fn ConstructionScript
  (Components|Box|SetBoxExtent (Variables|Default|GetBox) (Variables|Default|GetBoxSize) true))